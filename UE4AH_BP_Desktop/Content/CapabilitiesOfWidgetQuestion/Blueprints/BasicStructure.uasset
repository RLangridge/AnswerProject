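; Test RTS building actor with a world-space widget for buying infantry, tanks and infantry improvements with gold and minerals.
; The widget's purchase dispatchers deduct costs through RTSWidgetController.
; The controller's resource-change dispatchers trigger UpdateUI, which refreshes resource totals, caps and affordability-based button states.
; Tick rotates the widget to face the player pawn, keeping it readable.
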(event Custom|On%20Resources%20Gained
  ;[1 1 1] Update the UI whenever resources change
  (Utilities|UpdateUI))

(event Custom|On%20Purchase%20Infantry
  (Default|UpdateGold (Variables|ClassReferences|GetRTS%20Controller%20Reference) (* (Variables|BuildingStats|GetGold%20Cost%20Of%20Infantry) -1)))

(event Custom|On%20Purchase%20Infantry%20Improvement
  (Default|UpdateGold (Variables|ClassReferences|GetRTS%20Controller%20Reference) (* (Variables|BuildingStats|GetGold%20Cost%20To%20Improve%20Infantry) -1)))

(event Custom|On%20Purchase%20Tank
  (bind _rts_controller_reference (Variables|ClassReferences|GetRTS%20Controller%20Reference))
  ;[1 1 1] When someone presses a button on the UI, it will call an event dispatcher that will be associated with purchasing an item. We update the gold/mineral amount in the case of purchasing a tank. This in turn updates the UI based on our previous event dispatchers.
  (Default|UpdateGold _rts_controller_reference (* (Variables|BuildingStats|GetGold%20Cost%20Of%20Tanks) -1))
  (Default|UpdateMinerals _rts_controller_reference (* (Variables|BuildingStats|GetMineral%20Cost%20Of%20Tanks) -1)))

(event EventTick
  (params (DeltaSeconds :type Float%20%28single-precision%29))
  ;[1 1 1] We use this to rotate towards our camera. I would be using something akin to this in VR to constantly show the UI in the direction of the player
  (Transformation|SetWorldRotation (Variables|Default|GetWidget) (Math|Rotator|FindLookatRotation (Transformation|GetActorLocation) (Transformation|GetActorLocation (Variables|ClassReferences|GetPlayer%20Pawn%20Reference))) false false))

(event EventBeginPlay
  ;[1 1 1] For rotating the UI so we can always see it
  (Variables|ClassReferences|SetPlayer%20Pawn%20Reference (Game|Player|GetPlayerPawn 0))
  ;[1 1 1] I've stored some standard values such as gold and minerals for testing
  (bind _asrtswidget_controller (Utilities|Casting|CastToRTSWidgetController (Game|GetPlayerController 0)))
  (Variables|ClassReferences|SetRTS%20Controller%20Reference _asrtswidget_controller)
  ;[1 1 1] We also want a reference to the UI for the building
  (bind _asbuilding_ui (Utilities|Casting|CastToBuildingUI (UserInterface|GetUserWidgetObject (Variables|Default|GetWidget))))
  (Variables|ClassReferences|SetBuilding%20UI%20Reference _asbuilding_ui)
  (Utilities|UpdateUI
    (:Updated%20UI
      (EventDispatchers|BindEventtoUpdateGoldPerformed (Variables|ClassReferences|GetRTS%20Controller%20Reference) (delegate Custom|On%20Resources%20Gained))
      (EventDispatchers|BindEventtoUpdateMineralsPerformed (Variables|ClassReferences|GetRTS%20Controller%20Reference) (delegate Custom|On%20Resources%20Gained))
      (EventDispatchers|BindEventtoOnPurchaseInfantry (Variables|ClassReferences|GetBuilding%20UI%20Reference) (delegate Custom|On%20Purchase%20Infantry))
      (EventDispatchers|BindEventtoOnPurchaseInfantryImprovement (Variables|ClassReferences|GetBuilding%20UI%20Reference) (delegate Custom|On%20Purchase%20Infantry%20Improvement))
      (EventDispatchers|BindEventtoOnPurchaseTank (Variables|ClassReferences|GetBuilding%20UI%20Reference) (delegate Custom|On%20Purchase%20Tank)))))

(fn ConstructionScript)

(fn CanAffordTank
  (bind _rts_controller_reference (Variables|ClassReferences|GetRTS%20Controller%20Reference))
  (return (and (>= (Default|GetGold _rts_controller_reference) (Variables|BuildingStats|GetGold%20Cost%20Of%20Tanks)) (>= (Default|GetMinerals _rts_controller_reference) (Variables|BuildingStats|GetMineral%20Cost%20Of%20Tanks)))))

(fn CanAffordInfantry
  (return (>= (Default|GetGold (Variables|ClassReferences|GetRTS%20Controller%20Reference)) (Variables|BuildingStats|GetGold%20Cost%20Of%20Infantry))))

(fn CanAffordImproveInfantry
  (return (>= (Default|GetGold (Variables|ClassReferences|GetRTS%20Controller%20Reference)) (Variables|BuildingStats|GetGold%20Cost%20To%20Improve%20Infantry))))