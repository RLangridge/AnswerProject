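; BP_StaticMeshNameFinder is an example that searches an array of static meshes for elements whose names contain a given substring.
; On BeginPlay it fills the array with its ball, cube and wall meshes, then prints the display names of case-insensitive matches for "Cube".
; FindElementsWithNameSubstring does the filtering, testing each element's object name with Contains and returning the matches as a new array.
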(event EventBeginPlay
  (bind _array_of_static_meshes (Variables|MeshData|GetArray%20Of%20Static%20Meshes))
  (Utilities|Array|Add _array_of_static_meshes (Variables|Default|GetFloor_1_Ball))
  (Utilities|Array|Add _array_of_static_meshes (Variables|Default|GetFloor_1_Cube))
  (Utilities|Array|Add _array_of_static_meshes (Variables|Default|GetFloor_1_Wall))
  (bind _array_of_found_elements (CallFunction|FindElementswithNameSubstring "Cube" false))
  (for _array_element _array_of_found_elements
    (Development|PrintString (Utilities|GetDisplayName _array_element))))

(fn ConstructionScript)

(fn FindElementswithNameSubstring
  (params (Name%20Substring :type String) (bUseCase :type Boolean))
  (bind _found_elements (LocalVariables|GetFound%20Elements))
  (for _array_element (Variables|MeshData|GetArray%20Of%20Static%20Meshes)
    (if (Utilities|String|Contains (Utilities|GetObjectName _array_element) Name%20Substring bUseCase)
      (Utilities|Array|Add _found_elements _array_element)))
  (return _found_elements))