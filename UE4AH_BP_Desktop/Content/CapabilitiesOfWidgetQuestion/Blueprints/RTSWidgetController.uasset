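; RTSWidgetController is an example RTS controller that tracks the player's gold and minerals and shows the mouse cursor.
; A looping one-second timer started on BeginPlay adds to both resources as placeholder income.
; Update events clamp each resource between zero and its cap, then call event dispatchers so bound listeners learn of changes without polling.
; Getter functions expose the current amounts and caps.
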(event Custom|Update%20Gold
  (params (Gold%20Change :type Integer))
  ;[1 1 1] When our resources increase/decrease, we make a call to the relevant event to tell everything bound to that event that our resources have changed.
  (Variables|Default|SetGold (Math|Integer|Clamp(Integer) (+ Gold%20Change (Variables|Default|GetGold)) 0 (Variables|Default|GetGold%20Cap)))
  (Default|CallUpdateGoldPerformed))

(event Custom|Update%20Minerals
  (params (Mineral%20Change :type Integer))
  ;[1 1 1] When our resources increase/decrease, we make a call to the relevant event to tell everything bound to that event that our resources have changed.
  (Variables|Default|SetMinerals (Math|Integer|Clamp(Integer) (+ Mineral%20Change (Variables|Default|GetMinerals)) 0 (Variables|Default|GetMineral%20Cap)))
  (Default|CallUpdateMineralsPerformed))

(event Custom|Add%20Gold%20And%20Minerals
  ;[1 1 1] Gain gold/minerals every second. This is just as an example of course.
  (CallFunction|UpdateGold 3)
  (CallFunction|UpdateMinerals 2))

(event EventTick
  (params (DeltaSeconds :type Float%20%28single-precision%29)))

(event EventBeginPlay
  ;[1 1 1] Gain gold/minerals every second. This is just as an example of course.
  (Utilities|Time|SetTimerbyEvent (delegate Custom|Add%20Gold%20And%20Minerals) 1.0 true)
  (Variables|Default|SetbShowMouseCursor true))

(fn ConstructionScript)

(fn GetGold
  (return (Variables|Default|GetGold)))

(fn GetMinerals
  (return (Variables|Default|GetMinerals)))

(fn GetGoldCap
  (return (Variables|Default|GetGold%20Cap)))

(fn GetMineralCap
  (return (Variables|Default|GetMineral%20Cap)))