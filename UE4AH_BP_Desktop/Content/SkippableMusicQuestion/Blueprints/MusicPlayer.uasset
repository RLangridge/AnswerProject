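; MusicPlayer is a Blueprint that plays skippable background music from a list of tracks.
; On BeginPlay it registers itself as the background music reference on MusicPlayerController, then starts the current track.
; Next and previous events fade the audio out, wait out the fade, step the index, swap the sound and fade back in.
; SetMusicPointer wraps the index at both ends using modulo and a negative check.
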(event Custom|Go%20To%20Next%20Song
  (bind _fade_out_time (Variables|Sounds|GetFade%20Out%20Time))
  (Audio|Components|Audio|FadeOut (Variables|Default|GetAudio) _fade_out_time 0.0 :!class /Script/Engine.AudioComponent)
  (Utilities|FlowControl|Delay _fade_out_time)
  (Math|Integer|IncrementInt (Variables|Sounds|GetMusic%20Pointer)
    (:%20%20
      (CallFunction|SetMusicPointer)
      (Audio|Components|Audio|FadeIn (Variables|Default|GetAudio) (Variables|Sounds|GetFade%20In%20Time) 1.0 0.0 :!class /Script/Engine.AudioComponent))))

(event Custom|Go%20To%20Previous%20Song
  (bind _fade_out_time (Variables|Sounds|GetFade%20Out%20Time))
  (Audio|Components|Audio|FadeOut (Variables|Default|GetAudio) _fade_out_time 0.0 :!class /Script/Engine.AudioComponent)
  (Utilities|FlowControl|Delay _fade_out_time)
  (Math|Integer|DecrementInt (Variables|Sounds|GetMusic%20Pointer)
    (:%20%20
      (CallFunction|SetMusicPointer)
      (Audio|Components|Audio|FadeIn (Variables|Default|GetAudio) (Variables|Sounds|GetFade%20In%20Time) 1.0 0.0 :!class /Script/Engine.AudioComponent))))

(event Custom|Play%20Music
  (bind _audio (Variables|Default|GetAudio))
  (Audio|Components|Audio|SetSound _audio (Utilities|Array|Get(acopy) (Variables|Sounds|GetMusic%20To%20Play) (Variables|Sounds|GetMusic%20Pointer)))
  (Audio|Components|Audio|Play _audio 0.0))

(event EventBeginPlay
  (bind _asmusic_player_controller (Utilities|Casting|CastToMusicPlayerController (Game|GetPlayerController 0)))
  (Variables|/Game/SkippableMusicQuestion/Blueprints/MusicPlayerController.MusicPlayerController_C|SetBackground%20Music%20Reference _asmusic_player_controller self)
  (CallFunction|PlayMusic))

(fn ConstructionScript)

(fn SetMusicPointer
  (bind _output_get (Variables|Sounds|SetMusic%20Pointer (Math|Integer|SelectInt (- (Utilities|Array|Length (Variables|Sounds|GetMusic%20To%20Play)) 1) (Math|Integer|%(Integer) (Variables|Sounds|GetMusic%20Pointer) (Utilities|Array|Length (Variables|Sounds|GetMusic%20To%20Play))) (< (Variables|Sounds|GetMusic%20Pointer) 0))))
  (Audio|Components|Audio|SetSound (Variables|Default|GetAudio) (Utilities|Array|Get(acopy) (Variables|Sounds|GetMusic%20To%20Play) _output_get)))