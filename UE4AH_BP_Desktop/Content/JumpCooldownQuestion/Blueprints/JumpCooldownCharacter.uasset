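; JumpCooldownCharacter is a character Blueprint that limits jumping with a cooldown.
; On BeginPlay it caches the first player controller as a JumpCooldownPlayerController.
; A jump press passes a DoOnce gate, jumps and reports the cooldown duration to that controller through JumpHasOccurred.
; A Delay of the same duration then resets the gate, while releasing the input always calls StopJumping.
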(event EventBeginPlay
  (|CallParentFunction)
  (bind _asjump_cooldown_player_controller (Utilities|Casting|CastToJumpCooldownPlayerController (Game|GetPlayerController 0)))
  (Variables|Default|SetJump%20Controller%20Reference _asjump_cooldown_player_controller))

(event Input|ActionEvents|InputActionJump
  (params (Key :type Key%20Structure))
  (bind _jump_cooldown_duration (Variables|Default|GetJump%20Cooldown%20Duration))
  (:Pressed
    (Utilities|FlowControl|DoOnce false :!label _label
      (:Completed
        (Character|Jump)
        (Default|JumpHasOccurred (Variables|Default|GetJump%20Controller%20Reference) _jump_cooldown_duration)
        (Utilities|FlowControl|Delay _jump_cooldown_duration)
        (goto _label Reset))))
  (:Released
    (Character|StopJumping)))

(fn ConstructionScript
  (|CallParentFunction))